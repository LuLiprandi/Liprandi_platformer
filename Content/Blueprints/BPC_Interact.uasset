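; BPC_Interact is an interaction component that shows and hides an on-screen text prompt.
; On BeginPlay it creates a BPW_Interact widget and keeps a reference to it.
; ShowText copies the ChangeTxt variable into the widget's TxtInteract text and adds the widget to the viewport.
; UnshowText removes the widget from its parent, so the same instance is reused for each prompt.
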(event EventBeginPlay
  (bind _returnvalue (UserInterface|CreateWidget "/Game/Blueprints/BPW_Interact.BPW_Interact_C"))
  (Variables|Default|SetBPW_Interact _returnvalue))

(event EventTick
  (params (DeltaSeconds :type Float%20%28single-precision%29)))

(fn ShowText
  (bind _bpw_interact (Variables|Default|GetBPW_Interact))
  (Variables|/Script/UMG.TextBlock|SetText (Variables|/Game/Blueprints/BPW_Interact.BPW_Interact_C|GetTxtInteract _bpw_interact) (Variables|Default|GetChangeTxt))
  (UserInterface|Viewport|AddtoViewport _bpw_interact 0))

(fn UnshowText
  (Widget|RemovefromParent (Variables|Default|GetBPW_Interact)))