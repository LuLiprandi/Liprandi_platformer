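; BP_Button is an interactable button that controls a numbered light through the game instance.
; Overlapping it shows an "Interact with E" prompt through the BPCInteract component, and leaving hides it.
; BeginPlay caches BP_GameInstance, and the Activate event passes the button's LightControlledNumber to its UpdateLightState.
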(event EventBeginPlay
  (bind _asbp_game_instance (Utilities|Casting|CastToBP_GameInstance (Game|GetGameInstance)))
  (Variables|Default|SetAs%20BP%20Game%20Instance _asbp_game_instance))

(event Collision|EventActorBeginOverlap
  (params (OtherActor :type Actor%20Object%20Reference))
  (bind _bpc_interact (Variables|Default|GetBPC_Interact))
  (Variables|/Game/Blueprints/BPC_Interact.BPC_Interact_C|SetChangeTxt _bpc_interact "Interact with E")
  (Default|ShowText _bpc_interact))

(event EventTick
  (params (DeltaSeconds :type Float%20%28single-precision%29)))

(event EventActivate
  (Default|UpdateLightState (Variables|Default|GetAs%20BP%20Game%20Instance) (Variables|Default|GetLightControlledNumber)))

(event Collision|EventActorEndOverlap
  (params (OtherActor :type Actor%20Object%20Reference))
  (Default|UnshowText (Variables|Default|GetBPC_Interact)))

(fn ConstructionScript)