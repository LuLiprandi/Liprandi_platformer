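; BP_Light is a light actor whose point light visibility follows an on/off state stored in BP_GameInstance, looked up by the actor's Number.
; On BeginPlay it caches the game instance, binds UpdateLight to its OnLightToggle dispatcher and applies the current state immediately.
; Each toggle broadcast makes the light re-read its own state and show or hide the PointLight, so no Tick polling is used.
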(event Custom|UpdateLight
  ;[1 1 1] Lire Etat de la lumiere
  (bind _lightstate (Default|GetLightStatebyNumber (Variables|Default|GetAs%20BP%20Game%20Instance) (Variables|Default|GetNumber)))
  (Rendering|SetVisibility (Variables|Default|GetPointLight) _lightstate false))

(event EventBeginPlay
  ;[1 1 1] Lire Etat de la lumiere
  (bind _asbp_game_instance (Utilities|Casting|CastToBP_GameInstance (Game|GetGameInstance)))
  (bind _output_get (Variables|Default|SetAs%20BP%20Game%20Instance _asbp_game_instance))
  (EventDispatchers|BindEventtoOnLightToggle _output_get (delegate Custom|UpdateLight))
  (CallFunction|UpdateLight))

(event Collision|EventActorBeginOverlap
  (params (OtherActor :type Actor%20Object%20Reference)))

(event EventTick
  (params (DeltaSeconds :type Float%20%28single-precision%29)))

(fn ConstructionScript)