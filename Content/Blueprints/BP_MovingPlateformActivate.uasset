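; Moving platform actor that shuttles vertically between its starting height and a fixed height above it while IsMoving is true.
; BeginPlay stores the starting Z, then Tick moves the actor one unit per frame and flips direction through IsUp at either limit.
; Movement ignores delta time, so speed depends on frame rate.
; Nothing in this Blueprint sets IsMoving, and the overlap event is an empty stub.
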(event EventBeginPlay
  (Variables|Default|SetReturn%20Value%20Z (.z (Transformation|GetActorLocation))))

(event Collision|EventActorBeginOverlap
  (params (OtherActor :type Actor%20Object%20Reference)))

(event EventTick
  (params (DeltaSeconds :type Float%20%28single-precision%29))
  (bind _returnvalue (Transformation|GetActorLocation))
  (bind _returnvalue_2 (Transformation|GetActorLocation))
  (if (Variables|Default|GetIsMoving)
    (if (Variables|Default|GetIsUp)
      (Transformation|SetActorLocation (Math|Vector|MakeVector (.x _returnvalue_2) (.y _returnvalue_2) (+ (.z _returnvalue_2) -1.0)) false false)
      (Variables|Default|SetIsUp (<= (Variables|Default|GetReturn%20Value%20Z) (.z (Transformation|GetActorLocation))))
      (else
        (Transformation|SetActorLocation (Math|Vector|MakeVector (.x _returnvalue) (.y _returnvalue) (+ (.z _returnvalue) 1.0)) false false)
        (Variables|Default|SetIsUp (>= (.z (Transformation|GetActorLocation)) (+ (Variables|Default|GetReturn%20Value%20Z) 1255.0)))))))

(fn ConstructionScript)